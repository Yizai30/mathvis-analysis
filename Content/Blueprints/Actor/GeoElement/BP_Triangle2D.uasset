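; BP_Triangle2D is a 2D triangle geometry actor that can be dragged with the mouse and toggled as selected.
; Clicking the mesh disables pawn input, caches the cursor hit and opens a gate on Tick that moves the actor at that hit distance and offset.
; Every release toggles it in GI_Globe's GeoEffectActors, updating highlight and X/Y/Z rotate-button visibility, then restores input and closes the gate.
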(event OnClicked(GeoMeshComponent)
  (params (TouchedComponent :type Primitive%20Component%20Object%20Reference) (ButtonPressed :type Key%20Structure :default "None"))
  (bind _returnvalue (Game|GetPlayerController 0))
  (bind _returnvalue_2 (Game|GetPlayerController 0))
  (bind _hitresult (Game|Player|GetHitResultUnderCursorbyChannel _returnvalue_2 "TraceTypeQuery1" true))
  (bind (_locationx _locationy) (Game|Player|GetMousePosition _returnvalue))
  (bind _returnvalue_3 (Math|Vector2D|MakeVector2D _locationx _locationy))
  (bind (_bblockinghit _binitialoverlap _time _distance _location _impactpoint _normal _impactnormal _physmat _hitactor) (Collision|BreakHitResult _hitresult))
  (bind (_worldposition _worlddirection) (Class|GameplayStatics|DeprojectScreentoWorld _returnvalue _returnvalue_3))
  ;[0.15 0.15 0.15 0.5] 处理鼠标对图形的移动
  (Input|DisableInput (Game|Player|GetPlayerPawn 0) (Game|GetPlayerController 0))
  (Variables|Default|SetHitDistance _distance)
  (Variables|Default|SetHitLocation _location)
  (Variables|Default|SetHitActorLocation (Transformation|GetActorLocation _hitactor))
  (Utilities|FlowControl|Gate true) ; enters at Open
)

(event OnReleased(GeoMeshComponent)
  (params (TouchedComponent :type Primitive%20Component%20Object%20Reference) (ButtonReleased :type Key%20Structure :default "None"))
  (bind _returnvalue (Game|GetPlayerController 0))
  (bind _self self)
  (bind (_locationx _locationy) (Game|Player|GetMousePosition _returnvalue))
  (bind _returnvalue_2 (Math|Vector2D|MakeVector2D _locationx _locationy))
  (bind (_worldposition _worlddirection) (Class|GameplayStatics|DeprojectScreentoWorld _returnvalue _returnvalue_2))
  ;[0.15 0.15 0.15 0.5] 处理当前哪些图形被选中
  (Utilities|FlowControl|Sequence
    (:then_0
      (bind _asgi_globe (Utilities|Casting|CastToGI_Globe (Game|GetGameInstance)))
      (if (== (Utilities|Array|FindItem (Variables|/Game/Blueprints/GameInstance/GI_Globe.GI_Globe_C|GetGeoEffectActors _asgi_globe) _self) -1)
        ;;[0.15 0.15 0.15 0.5] 未找到该图形则添加
        (Utilities|Array|Add (Variables|/Game/Blueprints/GameInstance/GI_Globe.GI_Globe_C|GetGeoEffectActors _asgi_globe) _self)
        (Class|GeoEffectActor|HighlightActor)
        (bind _asgi_globe_2 (Utilities|Casting|CastToGI_Globe (Game|GetGameInstance)))
        (bind _output_get (Variables|Default|SetButtonRotateTriangle2D_X (Variables|/Game/Blueprints/GameInstance/GI_Globe.GI_Globe_C|GetButton_RotateTriangle2D_X _asgi_globe_2)))
        (Variables|/Script/UMG.Widget|SetVisibility _output_get "Visible")
        (bind _output_get_2 (Variables|Default|SetButtonRotateTriangle2D_Y (Variables|/Game/Blueprints/GameInstance/GI_Globe.GI_Globe_C|GetButton_RotateTriangle2D_Y _asgi_globe_2)))
        (Variables|/Script/UMG.Widget|SetVisibility _output_get_2 "Visible")
        (bind _output_get_3 (Variables|Default|SetButtonRotateTriangle2D_Z (Variables|/Game/Blueprints/GameInstance/GI_Globe.GI_Globe_C|GetButton_RotateTriangle2D_Z _asgi_globe_2)))
        (Variables|/Script/UMG.Widget|SetVisibility _output_get_3 "Visible")
        (else
          ;;[0.15 0.15 0.15 0.5] 找到则删除该图形
          (Utilities|Array|RemoveItem (Variables|/Game/Blueprints/GameInstance/GI_Globe.GI_Globe_C|GetGeoEffectActors _asgi_globe) _self)
          (Class|GeoEffectActor|UnHighlightActor)
          (Variables|/Script/UMG.Widget|SetVisibility (Variables|Default|GetButtonRotateTriangle2D_X) "Hidden")
          (Variables|/Script/UMG.Widget|SetVisibility (Variables|Default|GetButtonRotateTriangle2D_Y) "Hidden")
          (Variables|/Script/UMG.Widget|SetVisibility (Variables|Default|GetButtonRotateTriangle2D_Z) "Hidden")))
      (for _array_element (Variables|/Game/Blueprints/GameInstance/GI_Globe.GI_Globe_C|GetGeoEffectActors _asgi_globe)
        (Development|PrintString (Utilities|GetObjectName _array_element))))
    (:then_1
      (Input|EnableInput (Game|Player|GetPlayerPawn 0) (Game|GetPlayerController 0))
      ;[0.15 0.15 0.15 0.5] 处理鼠标对图形的移动
      (Utilities|FlowControl|Gate true) ; enters at Close
    )))

(event EventBeginPlay)

(event Collision|EventActorBeginOverlap
  (params (OtherActor :type Actor%20Object%20Reference)))

(event EventTick
  (params (DeltaSeconds :type Float%20%28single-precision%29))
  (bind _returnvalue (Game|GetPlayerController 0))
  (bind (_locationx _locationy) (Game|Player|GetMousePosition _returnvalue))
  (bind _returnvalue_2 (Math|Vector2D|MakeVector2D _locationx _locationy))
  (bind (_worldposition _worlddirection) (Class|GameplayStatics|DeprojectScreentoWorld _returnvalue _returnvalue_2))
  ;[0.15 0.15 0.15 0.5] 处理鼠标对图形的移动
  (Utilities|FlowControl|Gate true
    (:Exit
      (Transformation|SetActorLocation (+ (- (+ _worldposition (* _worlddirection (Variables|Default|GetHitDistance))) (Variables|Default|GetHitLocation)) (Variables|Default|GetHitActorLocation)) false false))))

(fn ConstructionScript)