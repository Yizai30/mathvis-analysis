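; BP_CamController is a player-driven camera pawn that moves, looks around and zooms through axis inputs.
; Forward and right movement follow only the control rotation's yaw, keeping travel horizontal, while Turn and LookUp feed controller yaw and pitch.
; MoveUp moves vertically using the Z component of the view's forward vector, so its effect depends on pitch.
; Zoom adjusts the spring arm length in large steps within a clamped range.
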(event EventBeginPlay)

(event Collision|EventActorBeginOverlap
  (params (OtherActor :type Actor%20Object%20Reference)))

(event EventTick
  (params (DeltaSeconds :type Float%20%28single-precision%29)))

(event Input|AxisEvents|InputAxisMoveForward
  (params (AxisValue :type Float%20%28single-precision%29))
  (Pawn|Input|AddMovementInput (Math|Vector|GetForwardVector (Math|Rotator|MakeRotator 0.0 0.0 (.Yaw (Math|Rotator|BreakRotator (Pawn|GetControlRotation :!class /Script/Engine.Pawn))))) AxisValue false))

(event Input|AxisEvents|InputAxisMoveRight
  (params (AxisValue :type Float%20%28single-precision%29))
  (Pawn|Input|AddMovementInput (Math|Vector|GetRightVector (Math|Rotator|MakeRotator 0.0 0.0 (.Yaw (Math|Rotator|BreakRotator (Pawn|GetControlRotation :!class /Script/Engine.Pawn))))) AxisValue false))

(event Input|AxisEvents|InputAxisTurn
  (params (AxisValue :type Float%20%28single-precision%29))
  (Pawn|Input|AddControllerYawInput AxisValue))

(event Input|AxisEvents|InputAxisLookUp
  (params (AxisValue :type Float%20%28single-precision%29))
  (Pawn|Input|AddControllerPitchInput AxisValue))

(event Input|AxisEvents|InputAxisMoveUp
  (params (AxisValue :type Float%20%28single-precision%29))
  (Pawn|Input|AddMovementInput (Math|Vector|MakeVector 0.0 0.0 (.z (Math|Vector|GetForwardVector (Pawn|GetControlRotation :!class /Script/Engine.Pawn)))) (* AxisValue 1e+02) false))

(event Input|AxisEvents|InputAxisZoom
  (params (AxisValue :type Float%20%28single-precision%29))
  (bind _springarm (Variables|Default|GetSpringArm))
  (Variables|/Script/Engine.SpringArmComponent|SetTargetArmLength _springarm (Math|Float|Clamp(Float) (+ (* AxisValue -1.5e+03) (Variables|/Script/Engine.SpringArmComponent|GetTargetArmLength _springarm)) 0.0 1.985e+05)))

(fn ConstructionScript)