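; GI_Globe is a Game Instance Blueprint that records timestamped transforms of effect actors (MVEffectActor) in shared lookup maps.
; AddGeoWithTimestamp writes each entry into two indexes: timestamp to a list of geo transforms, and effect actor to a list of time-transform pairs.
; Each write finds the existing struct-wrapped list, appends to it and adds it back to the map under the same key.
; A debug print of list length is left unconnected.
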(fn AddGeowithTimestamp
  (params (Timestamp :type Float%20%28double-precision%29) (GeoTransform :type DS%20MV%20Transfrom%20Structure))
  (bind (_mveffectactor _transform) (Utilities|Struct|BreakDS_MVTransfrom GeoTransform))
  (Variables|Default|SetTimestamp Timestamp)
  (Utilities|FlowControl|Sequence
    (:then_0
      ;[0.15 0.15 0.15 0.5] [Time]映射到[DS_GeoTransform]
      (bind _output_get (Variables|Default|SetGeoTransfromList (Utilities|Struct|BreakDS_GeoTransformList (.Value (Utilities|Map|Find (Variables|Default|GetTimeToGeoTransformListMap) (Variables|Default|GetTimestamp))))))
      (Utilities|Array|Add _output_get GeoTransform)
      (Utilities|Map|Add (Variables|Default|GetTimeToGeoTransformListMap) (Variables|Default|GetTimestamp) (Utilities|Struct|MakeDS_GeoTransformList (Variables|Default|GetGeoTransfromList))))
    (:then_1
      ;[0.15 0.15 0.15 0.5] [GeoEffectActor]映射到[DS_TimeTransform]
      (bind _output_get_2 (Variables|Default|SetTimeTransformList (Utilities|Struct|BreakDS_TimeTransformList (.Value (Utilities|Map|Find (Variables|Default|GetMVEleToTimeTransformListMap) _mveffectactor)))))
      (Utilities|Array|Add _output_get_2 (Utilities|Struct|MakeDS_TimeTransform (Variables|Default|GetTimestamp) _transform))
      (Utilities|Map|Add (Variables|Default|GetMVEleToTimeTransformListMap) _mveffectactor (Utilities|Struct|MakeDS_TimeTransformList (Variables|Default|GetTimeTransformList))))))